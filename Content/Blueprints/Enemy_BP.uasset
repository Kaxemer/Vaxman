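; Enemy for a Vaxman game that wanders randomly, clones itself periodically and destroys itself when its sphere hits Vaxman_BP.
; BeginPlay binds the state-change event and idles briefly before switching to Hunt.
; UpdateMovementTarget, run on state changes and a fast repeating timer, stops AI movement in Idle and otherwise moves to a random reachable point nearby.
; A slower looping timer spawns another Enemy_BP at its transform, so the population multiplies.
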(event OnComponentHit(Sphere)
  (params (HitComponent :type Primitive%20Component%20Object%20Reference) (OtherActor :type Actor%20Object%20Reference) (OtherComp :type Primitive%20Component%20Object%20Reference) (NormalImpulse :type Vector :default "0, 0, 0") (Hit :type Hit%20Result%20Structure%20%28by%20ref%29))
  (Utilities|Casting|CastToVaxman_BP OtherActor)
  (Actor|DestroyActor self))

(event Custom|Event%20State%20Changed%20Setup
  (EventDispatchers|BindEventtoStateChangedEvent (delegate Custom|Event%20State%20Changed)))

(event Custom|Event%20State%20Changed
  (params (NewState :type EEnemyState%20Enum :default "Default"))
  (CallFunction|UpdateMovementTarget))

(event Custom|RandomMovement
  (CallFunction|UpdateMovementTarget))

(event Custom|Replicate
  (Game|SpawnActorfromClass "Enemy_BP_C" (Transformation|GetActorTransform) "AlwaysSpawn" 0 0))

(event EventBeginPlay
  (CallFunction|EventStateChangedSetup)
  (Class|EnemyPawn|Idle)
  (Utilities|FlowControl|Delay 2.0)
  (Utilities|Time|SetTimerbyEvent (delegate Custom|Replicate) 3e+01 true)
  (Class|EnemyPawn|Hunt)
  (Utilities|Time|SetTimerbyEvent (delegate Custom|RandomMovement) 0.12 true))

(fn ConstructionScript)

(fn UpdateMovementTarget
  (LocalVariables|SetAI%20Controller (AI|GetAIController (Pawn|GetController)))
  (switch Utilities|FlowControl|Switch|SwitchonEEnemyState (Variables|Default|GetState)
    (:Default
      (AI|Navigation|MovetoLocation (LocalVariables|GetAI%20Controller) (.RandomLocation (AI|Navigation|GetRandomReachablePointinRadius (Transformation|GetActorLocation) 4e+03 0 0)) 0.0 true true false true 0))
    (:Idle
      (AI|Navigation|StopMovement (LocalVariables|GetAI%20Controller)))))