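; Game mode for Vaxman that sets up the match and decides win or loss from pellet and ghost counts.
; On BeginPlay it blends the view to the first level CameraActor, waits briefly, then starts two looping timers and unfreezes the player.
; The timers poll actor counts: no pellets left wins, too many ghosts loses, checked far less often.
; Both outcomes print a message and restart the game after a short delay.
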(event Custom|Setup%20Camera
  (bind _outactors (Actor|GetAllActorsOfClass "/Script/Engine.CameraActor"))
  (Game|Player|SetViewTargetwithBlend (Game|GetPlayerController 0) (Utilities|Array|Get(acopy) _outactors) 1.0 "VTBlend_Linear" 0.0 false))

(event Custom|CheckGhosts
  (bind _outactors (Actor|GetAllActorsOfClass "/Game/Blueprints/Enemy_BP.Enemy_BP_C"))
  (if (>= (Utilities|Array|Length _outactors) 128)
    (Development|PrintString "Too Many Ghosts. You Lose!" true true "(R=1.000000,G=0.000000,B=0.342600,A=1.000000)")
    (Utilities|FlowControl|Delay 2.0)
    (Class|GameMode|RestartGame)))

(event Custom|CheckPellets
  (bind _outactors (Actor|GetAllActorsOfClass "/Game/Blueprints/Pellet_BP.Pellet_BP_C"))
  (if (<= (Utilities|Array|Length _outactors) 0)
    (Development|PrintString "All Pellets Eaten! You win.")
    (Utilities|FlowControl|Delay 2.0)
    (Class|GameMode|RestartGame)))

(event EventBeginPlay
  (CallFunction|SetupCamera)
  (Utilities|FlowControl|Delay 2.0)
  (Utilities|Time|SetTimerbyEvent (delegate Custom|CheckGhosts) 3e+01 true)
  (Utilities|Time|SetTimerbyEvent (delegate Custom|CheckPellets) 0.1 true)
  (bind _asvaxman_bp (Utilities|Casting|CastToVaxman_BP (Game|Player|GetPlayerPawn 0)))
  (Class|VaxmanPawn|SetFrozen _asvaxman_bp false))

(fn ConstructionScript)